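; BP_BuildableArea is a clickable build spot for towers that opens and closes a build menu.
; Clicking its Box toggles the plus sign and either creates BP_BuildMenuWidget at the area's projected screen position or removes it.
; The area passes itself and its location to the menu as the build target.
; Tick polls the menu's HasTower flag into IsTower, which blocks further clicks once a tower exists.
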(event OnClicked(Box)
  (params (TouchedComponent :type Primitive%20Component%20Object%20Reference) (ButtonPressed :type Key%20Structure :default "None"))
  (if (not (Variables|Default|GetIsTower))
    (if (Variables|Default|GetIsPlusSignVisible)
      (Variables|Default|SetIsPlusSignVisible false)
      (else
        (Variables|Default|SetIsPlusSignVisible true)))
    (Rendering|SetVisibility (Variables|Default|GetPlusSign) (Variables|Default|GetIsPlusSignVisible) false)
    (if (Variables|Default|GetIsPlusSignVisible)
      (bind _returnvalue (UserInterface|CreateWidget "/Game/Blueprints/BP_BuildMenuWidget.BP_BuildMenuWidget_C" (Game|GetPlayerController 0)))
      (Variables|Default|SetMenu _returnvalue)
      (Variables|/Game/Blueprints/BP_BuildMenuWidget.BP_BuildMenuWidget_C|SetTargetBuildableArea (Variables|Default|GetMenu) self)
      (Variables|/Game/Blueprints/BP_BuildMenuWidget.BP_BuildMenuWidget_C|SetBuildLocation (Variables|Default|GetMenu) (Transformation|GetActorLocation))
      (UserInterface|Viewport|AddtoViewport (Variables|Default|GetMenu) 0)
      (Class|UserWidget|SetPositioninViewport (Variables|Default|GetMenu) (.ScreenPosition (Class|GameplayStatics|ProjectWorldtoScreen (Game|GetPlayerController 0) (Transformation|GetActorLocation) false)) true)
      (else
        (Widget|RemovefromParent (Variables|Default|GetMenu))))))

(event EventBeginPlay)

(event Collision|EventActorBeginOverlap
  (params (OtherActor :type Actor%20Object%20Reference)))

(event EventTick
  (params (DeltaSeconds :type Float%20%28single-precision%29))
  (bind _menu (Variables|Default|GetMenu))
  (if (Utilities|IsValid _menu)
    (Variables|Default|SetIsTower (Variables|/Game/Blueprints/BP_BuildMenuWidget.BP_BuildMenuWidget_C|GetHasTower _menu))))

(fn ConstructionScript)