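; BP_MonsterPaperFlipbookActor is a monster flipbook actor with an HP bar widget and a toggleable pin mark.
; BeginPlay caches the WB_MonsterHPBar from the HPBar component and hides PinMark.
; Tick pushes the HP to MAXHP ratio into the widget every frame.
; The SetPinMarkVisibility event shows or hides the mark on demand.
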(event EventBeginPlay
  (bind _aswb_monster_hpbar (Utilities|Casting|CastToWB_MonsterHPBar (UserInterface|GetUserWidgetObject (Variables|Default|GetHPBar))))
  (Variables|Default|SetAs%20WB%20Monster%20HPBar _aswb_monster_hpbar)
  (Rendering|SetVisibility (Variables|Default|GetPinMark) false false))

(event Collision|EventActorBeginOverlap
  (params (OtherActor :type Actor%20Object%20Reference)))

(event EventTick
  (params (DeltaSeconds :type Float%20%28single-precision%29))
  (Variables|/Game/Blueprints/WidgetBlueprint/WB_MonsterHPBar.WB_MonsterHPBar_C|SetHPValue (Variables|Default|GetAs%20WB%20Monster%20HPBar) (/ (Variables|Default|GetHP) (Variables|Default|GetMAX_HP))))

(event EventSetPinMarkVisibility
  (params (IsVisable :type Boolean))
  (Rendering|SetVisibility (Variables|Default|GetPinMark) IsVisable false))

(fn ConstructionScript)